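; TileFloor is a Blueprint that builds a rectangular floor from a repeated tile mesh.
; Its construction script loops over MeshTileX by MeshTileY and adds one instance per cell to the FloorTile instanced mesh component.
; Spacing comes from the mesh's bounding box size, so tiles sit edge to edge at unit scale, with an offset fixed at zero.
; The event graph holds only disabled placeholder events.
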(fn `UserConstructionScript`
  (bind (_min _max) (break `Box` (`StaticMesh.GetBoundingBox` (`StaticMeshComponent.StaticMesh` (`self.FloorTile`)))))
  (bind _output_get (set `self.Offset` 0.0))
  (for _index (range (`self.MeshTileX`))
    (for _index_2 (range (`self.MeshTileY`))
      (`InstancedStaticMeshComponent.AddInstance` (`self.FloorTile`) (`KismetMathLibrary.MakeTransform` (`KismetMathLibrary.MakeVector` (- (* _index (.x (- _max _min))) _output_get) (- (* _index_2 (.y (- _max _min))) _output_get)))))))