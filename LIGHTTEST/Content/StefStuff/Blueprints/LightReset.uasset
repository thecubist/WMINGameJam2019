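; LightReset is a trigger actor that resets the red and blue values and all buttons while both players are inside it.
; Overlap events track FirstPersonCharacter and Player2 with separate flags.
; While both are set, Tick zeroes Red and Blue on the Global game instance, calls ResetButton on every Buttons actor and prints a debug message, repeating every frame.
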(event `self.ReceiveBeginPlay`
  (set `self.player1Detected` false)
  (set `self.player2Detected` false))

(event `self.ReceiveActorBeginOverlap`
  (params (OtherActor :type "Actor Object Reference"))
  (`|ExecutionSequence`
    (:`then_0`
      (cast `/Game/FirstPersonBP/Blueprints/FirstPersonCharacter` OtherActor)
      (set `self.player1Detected` true))
    (:`then_1`
      (cast `/Game/FirstPersonBP/Blueprints/Player2` OtherActor)
      (set `self.player2Detected` true))))

(event `self.ReceiveTick`
  (params (DeltaSeconds :type "Float (single-precision)"))
  (if (and (`self.player1Detected`) (`self.player2Detected`))
    (bind _asglobal (cast `/Game/BluePrints/Global` (`GameplayStatics.GetGameInstance`)))
    (set `/Game/BluePrints/Global.Red` 0 _asglobal)
    (set `/Game/BluePrints/Global.Blue` 0 _asglobal)
    (bind _outactors (`GameplayStatics.GetAllActorsOfClass` "/Game/BluePrints/Buttons/Buttons.Buttons_C"))
    (for _array_element _outactors
      (`/Game/BluePrints/Buttons/Buttons.ResetButton` _array_element))
    (`KismetSystemLibrary.PrintString` "reset buttons")))

(event `self.ReceiveActorEndOverlap`
  (params (OtherActor :type "Actor Object Reference"))
  (`|ExecutionSequence`
    (:`then_0`
      (cast `/Game/FirstPersonBP/Blueprints/FirstPersonCharacter` OtherActor)
      (set `self.player1Detected` false))
    (:`then_1`
      (cast `/Game/FirstPersonBP/Blueprints/Player2` OtherActor)
      (set `self.player2Detected` false))))

(fn `UserConstructionScript`)