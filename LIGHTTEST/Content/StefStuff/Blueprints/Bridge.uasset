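; Bridge actor pairing a PhaseMesh with a separate collidable PhysicsMesh, apparently for a phasing bridge.
; On BeginPlay, PhysicsMesh copies PhaseMesh's static mesh, scales slightly larger, and parks far below at the same truncated X/Y as its hidden location.
; Tick and GetReferences are empty, and a disconnected HitboxSize branch that would move the hitbox never runs, so nothing here brings the collision back.
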(event `self.ReceiveBeginPlay`
  (bind _physicsmesh (`self.PhysicsMesh`))
  (bind _phasemesh (`self.PhaseMesh`))
  ;[1 1 1] matching the model of the collidable mesh and moving it to its "hidden" location
  (`StaticMeshComponent.SetStaticMesh` _physicsmesh (`StaticMeshComponent.StaticMesh` _phasemesh))
  (`SceneComponent.K2_SetWorldLocation` _physicsmesh (`KismetMathLibrary.Conv_IntVectorToVector` (make `IntVector` (`KismetMathLibrary.FTrunc` (.x (`SceneComponent.K2_GetComponentLocation` _phasemesh))) (`KismetMathLibrary.FTrunc` (.y (`SceneComponent.K2_GetComponentLocation` _phasemesh))) -10000)) false false)
  (`SceneComponent.SetWorldScale3D` _physicsmesh (+ (`SceneComponent.K2_GetComponentScale` _phasemesh) 0.05)))

(event `self.ReceiveTick`
  (params (DeltaSeconds :type "Float (single-precision)")))

(fn `GetReferences`)

(fn `UserConstructionScript`)