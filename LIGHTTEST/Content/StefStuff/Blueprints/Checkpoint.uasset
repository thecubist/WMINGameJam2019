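; Checkpoint actor that detects overlaps from the two player character classes, FirstPersonCharacter and Player2, but does not yet act on them.
; On overlap, it casts to each class in turn and checks RespawnPointIsSelf, with nothing wired after the check.
; An offset position from the actor's location and SpawnPointYOffset, plus a RespawnPointOverride variable, sit unconnected in the graph, so no respawn point is set.
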(event `self.ReceiveActorBeginOverlap`
  (params (OtherActor :type "Actor Object Reference"))
  (bind _respawnpointisself (`self.RespawnPointIsSelf`))
  (`|ExecutionSequence`
    (:`then_0`
      (cast `/Game/FirstPersonBP/Blueprints/FirstPersonCharacter` OtherActor)
      (if _respawnpointisself
        _))
    (:`then_1`
      (cast `/Game/FirstPersonBP/Blueprints/Player2` OtherActor)
      (if _respawnpointisself
        _))))

(fn `UserConstructionScript`)