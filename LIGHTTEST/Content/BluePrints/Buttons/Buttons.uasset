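; Button actor Blueprint with a light that can be switched between red, white and blue.
; The construction script creates a dynamic material instance on the Light component and stores it.
; The ChangeRed, ChangeWhite and ChangeBlue events set that material's LightColour parameter and update three mutually exclusive booleans that record the current colour.
; Nothing in this Blueprint calls these events.
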(event `self.ReceiveTick`
  (params (DeltaSeconds :type "Float (single-precision)")))

(event `ChangeRed`
  (`MaterialInstanceDynamic.SetVectorParameterValue` (`self.DynamicMat`) "LightColour" (struct :`R` 1.0 :`B` 0.072084 :`A` 1.0))
  (set `self.red` true)
  (set `self.white` false)
  (set `self.blue` false))

(event `ChangeWhite`
  (`MaterialInstanceDynamic.SetVectorParameterValue` (`self.DynamicMat`) "LightColour" (struct :`R` 1.0 :`G` 1.0 :`B` 1.0 :`A` 1.0))
  (set `self.white` true)
  (set `self.red` false)
  (set `self.blue` false))

(event `ChangeBlue`
  (`MaterialInstanceDynamic.SetVectorParameterValue` (`self.DynamicMat`) "LightColour" (struct :`G` 0.35644 :`B` 1.0 :`A` 1.0))
  (set `self.blue` true)
  (set `self.white` false)
  (set `self.red` false))

(fn `UserConstructionScript`
  (bind _returnvalue (`PrimitiveComponent.CreateDynamicMaterialInstance` (`self.Light`) 0 null "None"))
  (set `self.DynamicMat` _returnvalue))